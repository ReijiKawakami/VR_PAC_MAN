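; End-screen HUD for a VR Pac-Man game that shows the result image and posts the player's score online.
; DrawHUD scales the End texture to screen width, centers it partly vertically and overlays a "ReStart" hit box.
; BeginPlay posts the GameInstance's Twitter account and time-weighted score as JSON to a Heroku endpoint, ignoring the response.
; HitBoxClick opens GameStartMap only for "Start", which does not match the hit box name.
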(event Custom|OnGetResult
  ;[1 1 1] PostData
)

(event EventDrawHUD
  (params (SizeX :type Integer) (SizeY :type Integer))
  ;[1 1 1] Draw HUD
  (Variables|Default|SetScale (/ (Math|Conversions|ToFloat(Integer) SizeX) 9.6e+02))
  (Canvas|DrawTexture "/Game/GameEnd/Textures/End.End" 0.0 (/ (- (Math|Conversions|ToFloat(Integer) SizeY) (* (Variables|Default|GetScale) 6.4e+02)) 3.0) 9.6e+02 6.4e+02 0.0 0.0 1.0 1.0 "(R=1.000000,G=1.000000,B=1.000000,A=1.000000)" "BLEND_Opaque" (Variables|Default|GetScale))
  (Class|HUD|AddHitBox (+ (* (Math|Vector2D|MakeVector2D 375.0 389.0) (Variables|Default|GetScale)) (Math|Vector2D|MakeVector2D 0.0 (/ (- (Math|Conversions|ToFloat(Integer) SizeY) (* (Variables|Default|GetScale) 6.4e+02)) 3.0))) (* (Math|Vector2D|MakeVector2D 2.5e+02 58.0) (Variables|Default|GetScale)) "ReStart" false))

(event EventHitBoxClick
  (params (BoxName :type Name))
  ;[1 1 1] HitBoxClicked
  (switch name BoxName
    (:Start
      (Game|OpenLevel(byName) "GameStartMap"))))

(event EventBeginPlay
  ;[1 1 1] PostData
  (Variables|Default|SetJsonData (Class|JsonFieldData|Create))
  (bind _asvrpac_man_game_instance (Utilities|Casting|CastToVRPacManGameInstance (Game|GetGameInstance)))
  (Class|JsonFieldData|PostRequest (Class|JsonFieldData|SetObjectArray (Variables|Default|GetJsonData) "score" (Utilities|Array|MakeArray (Class|JsonFieldData|SetString (Class|JsonFieldData|SetString (Class|JsonFieldData|Create) "name" (Variables|/Game/VRPacManGameInstance.VRPacManGameInstance_C|GetTwitterAccount _asvrpac_man_game_instance)) "score" (Utilities|String|ToString(Integer) (+ (Variables|/Game/VRPacManGameInstance.VRPacManGameInstance_C|GetScore _asvrpac_man_game_instance) (* (Variables|/Game/VRPacManGameInstance.VRPacManGameInstance_C|GetTimes _asvrpac_man_game_instance) 4)))))) "https://supermarche-madame-4325.herokuapp.com/AddUser")
  (EventDispatchers|BindEventtoOnGetResult (Variables|Default|GetJsonData) (delegate Custom|OnGetResult)))

(fn ConstructionScript)